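; Wave manager that spawns timed enemy waves from a data asset on BeginPlay, moving on without waiting for kills.
; Nested loops built from wire re-entry and Delays step through waves, enemy groups and counts, playing a sound for boss waves.
; A random stream sets spawn spacing and Y position between LeftMax and RightMax markers.
; Each enemy can receive a pickup class to drop on death.
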(event Custom|SpawnNextWave
  (bind _currentwaveindex (Variables|Default|GetCurrentWaveIndex))
  (bind _waves (Variables|Default|GetWaves))
  (bind _leftmax (Variables|Default|GetLeftMax))
  (bind _returnvalue (Transformation|GetWorldLocation _leftmax))
  (bind _output (Utilities|Array|Get(acopy) _waves _currentwaveindex))
  (Math|Integer|IncrementInt (Variables|Default|GetCurrentWaveIndex)
    (:%20%20
      (if (Utilities|Array|IsValidIndex _waves (Variables|Default|GetCurrentWaveIndex))
        (Utilities|FlowControl|Delay (.intialdelay _output))
        (Development|PrintString (Utilities|String|Append "CurrentWaveIndex:" (Utilities|String|ToString(Integer) (Variables|Default|GetCurrentWaveIndex))))
        (if (.isbosswave _output)
          (Audio|PlaySound2D "/Game/Mini_Retro_music/CUE/LOOPS/CUE_Mega_G_loop_Cue.CUE_Mega_G_loop_Cue" 1.0 1.0 0.0 0 0))
        (Variables|Default|SetCurrentEnemiesData (.enemies _output))
        (bind _output_get (Variables|Default|SetCurrentEnemiesIndex -1))
        (bind _result (Math|Integer|IncrementInt _output_get)
          (:%20%20
            (Development|PrintString (Utilities|String|Append "CurrentEnemyIndex" (Utilities|String|ToString(Integer) (Variables|Default|GetCurrentEnemiesIndex))))
            (if (Utilities|Array|IsValidIndex (Variables|Default|GetCurrentEnemiesData) _result)
              (Variables|Default|SetMaxEnemyCount (.enemycount (Utilities|Array|Get(acopy) (Variables|Default|GetCurrentEnemiesData) (Variables|Default|GetCurrentEnemiesIndex))))
              (bind _output_get_2 (Variables|Default|SetCurrentEnemyCount 0))
              (if (< _output_get_2 (Variables|Default|GetMaxEnemyCount)) :!label _label
                (Game|SpawnActorfromClass (.enemyclass (Utilities|Array|Get(acopy) (Variables|Default|GetCurrentEnemiesData) (Variables|Default|GetCurrentEnemiesIndex))) (Math|Transform|MakeTransform (Math|Vector|MakeVector (.x _returnvalue) (Math|Random|RandomFloatinRangefromStream (Variables|Default|GetStream) (.y _returnvalue) (.y (Transformation|GetWorldLocation (Variables|Default|GetRightMax)))) (.z _returnvalue)) "0.000000,180.000000,0.000000" "1.000000,1.000000,1.000000") "AlwaysSpawn" "MultiplyWithRoot" 0 (select (.candroppickup (Utilities|Array|Get(acopy) (Variables|Default|GetCurrentEnemiesData) (Variables|Default|GetCurrentEnemiesIndex))) (.pickupclass (Utilities|Array|Get(acopy) (Variables|Default|GetCurrentEnemiesData) (Variables|Default|GetCurrentEnemiesIndex))) 0) 0)
                (Math|Integer|IncrementInt (Variables|Default|GetCurrentEnemyCount)
                  (:%20%20
                    (Utilities|FlowControl|Delay (Math|Random|RandomFloatinRangefromStream (Variables|Default|GetStream) 1.0 2.0))
                    (goto _label)))
                (else
                  (Development|PrintString "Spawn Next Enemy In Current wave")
                  (CallFunction|SpawnNextEnemiesinCurrentWave)))
              (else
                (CallFunction|SpawnNextWave)))))
        (else
          (Development|PrintString "No MoreWaves In Datat Asset To Spawn"))))))

(event Custom|StartSpawningWaves
  (bind _currentwaveindex (Variables|Default|GetCurrentWaveIndex))
  (bind _waves (Variables|Default|GetWaves))
  (bind _leftmax (Variables|Default|GetLeftMax))
  (bind _returnvalue (Transformation|GetWorldLocation _leftmax))
  (bind _output (Utilities|Array|Get(acopy) _waves _currentwaveindex))
  (if (Utilities|Array|IsValidIndex _waves (Variables|Default|GetCurrentWaveIndex))
    (Utilities|FlowControl|Delay (.intialdelay _output))
    (Development|PrintString (Utilities|String|Append "CurrentWaveIndex:" (Utilities|String|ToString(Integer) (Variables|Default|GetCurrentWaveIndex))))
    (if (.isbosswave _output)
      (Audio|PlaySound2D "/Game/Mini_Retro_music/CUE/LOOPS/CUE_Mega_G_loop_Cue.CUE_Mega_G_loop_Cue" 1.0 1.0 0.0 0 0))
    (Variables|Default|SetCurrentEnemiesData (.enemies _output))
    (bind _output_get (Variables|Default|SetCurrentEnemiesIndex -1))
    (bind _result (Math|Integer|IncrementInt _output_get)
      (:%20%20
        (Development|PrintString (Utilities|String|Append "CurrentEnemyIndex" (Utilities|String|ToString(Integer) (Variables|Default|GetCurrentEnemiesIndex))))
        (if (Utilities|Array|IsValidIndex (Variables|Default|GetCurrentEnemiesData) _result)
          (Variables|Default|SetMaxEnemyCount (.enemycount (Utilities|Array|Get(acopy) (Variables|Default|GetCurrentEnemiesData) (Variables|Default|GetCurrentEnemiesIndex))))
          (bind _output_get_2 (Variables|Default|SetCurrentEnemyCount 0))
          (if (< _output_get_2 (Variables|Default|GetMaxEnemyCount)) :!label _label
            (Game|SpawnActorfromClass (.enemyclass (Utilities|Array|Get(acopy) (Variables|Default|GetCurrentEnemiesData) (Variables|Default|GetCurrentEnemiesIndex))) (Math|Transform|MakeTransform (Math|Vector|MakeVector (.x _returnvalue) (Math|Random|RandomFloatinRangefromStream (Variables|Default|GetStream) (.y _returnvalue) (.y (Transformation|GetWorldLocation (Variables|Default|GetRightMax)))) (.z _returnvalue)) "0.000000,180.000000,0.000000" "1.000000,1.000000,1.000000") "AlwaysSpawn" "MultiplyWithRoot" 0 (select (.candroppickup (Utilities|Array|Get(acopy) (Variables|Default|GetCurrentEnemiesData) (Variables|Default|GetCurrentEnemiesIndex))) (.pickupclass (Utilities|Array|Get(acopy) (Variables|Default|GetCurrentEnemiesData) (Variables|Default|GetCurrentEnemiesIndex))) 0) 0)
            (Math|Integer|IncrementInt (Variables|Default|GetCurrentEnemyCount)
              (:%20%20
                (Utilities|FlowControl|Delay (Math|Random|RandomFloatinRangefromStream (Variables|Default|GetStream) 1.0 2.0))
                (goto _label)))
            (else
              (Development|PrintString "Spawn Next Enemy In Current wave")
              (CallFunction|SpawnNextEnemiesinCurrentWave)))
          (else
            (CallFunction|SpawnNextWave)))))
    (else
      (Development|PrintString "No MoreWaves In Datat Asset To Spawn"))))

(event Custom|SpawnNextEnemiesInCurrentWave
  (bind _currentenemiesdata (Variables|Default|GetCurrentEnemiesData))
  (bind _currentenemiesindex (Variables|Default|GetCurrentEnemiesIndex))
  (bind _leftmax (Variables|Default|GetLeftMax))
  (bind _returnvalue (Transformation|GetWorldLocation _leftmax))
  (bind _output (Utilities|Array|Get(acopy) _currentenemiesdata _currentenemiesindex))
  (bind _result (Math|Integer|IncrementInt (stale Custom|SpawnNextWave _output_get))
    (:%20%20
      (Development|PrintString (Utilities|String|Append "CurrentEnemyIndex" (Utilities|String|ToString(Integer) (Variables|Default|GetCurrentEnemiesIndex))))
      (if (Utilities|Array|IsValidIndex _currentenemiesdata _result)
        (Variables|Default|SetMaxEnemyCount (.enemycount _output))
        (bind _output_get (Variables|Default|SetCurrentEnemyCount 0))
        (if (< _output_get (Variables|Default|GetMaxEnemyCount)) :!label _label
          (Game|SpawnActorfromClass (.enemyclass _output) (Math|Transform|MakeTransform (Math|Vector|MakeVector (.x _returnvalue) (Math|Random|RandomFloatinRangefromStream (Variables|Default|GetStream) (.y _returnvalue) (.y (Transformation|GetWorldLocation (Variables|Default|GetRightMax)))) (.z _returnvalue)) "0.000000,180.000000,0.000000" "1.000000,1.000000,1.000000") "AlwaysSpawn" "MultiplyWithRoot" 0 (select (.candroppickup _output) (.pickupclass _output) 0) 0)
          (Math|Integer|IncrementInt (Variables|Default|GetCurrentEnemyCount)
            (:%20%20
              (Utilities|FlowControl|Delay (Math|Random|RandomFloatinRangefromStream (Variables|Default|GetStream) 1.0 2.0))
              (goto _label)))
          (else
            (Development|PrintString "Spawn Next Enemy In Current wave")
            (CallFunction|SpawnNextEnemiesinCurrentWave)))
        (else
          (CallFunction|SpawnNextWave))))))

(event EventBeginPlay
  (Class|KismetMathLibrary|ResetRandomStream (Variables|Default|GetStream))
  (Variables|Default|SetWaves (Variables|/Game/Blueprints/PDA_SetOfWaves.PDA_SetOfWaves_C|GetWaves (Variables|Default|GetWavesDataAsset)))
  (Variables|Default|SetNumberOfWaves (Utilities|Array|Length (Variables|/Game/Blueprints/PDA_SetOfWaves.PDA_SetOfWaves_C|GetWaves (Variables|Default|GetWavesDataAsset))))
  (CallFunction|StartSpawningWaves))

(fn ConstructionScript)