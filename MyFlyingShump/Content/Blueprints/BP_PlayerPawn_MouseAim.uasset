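; Player pawn for a top-down shooter that moves on world axes through Enhanced Input and yaws each Tick toward a cursor/touch trace point.
; Primary fire uses one of three debug-key-switched modes: minigun, missiles from two alternating muzzles, or fanned bullet spray.
; Damage reduces health with camera shake and a red overlay flash; at zero, it possesses a new pawn spawned at PlayerStart and destroys itself.
; HUD updates are stubs.
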(event Custom|BeginFire
  (Audio|PlaySound2D "/Game/Sci-Fi_Shots_Pack2_Game_Of_Weapons/Cue/SciFi_Shot_P2__122__Cue.SciFi_Shot_P2__122__Cue" 1.0 1.0 0.0 0 0)
  (Game|SpawnActorfromClass "/Game/Blueprints/BP_Bullet_2D_Player.BP_Bullet_2D_Player_C" (Math|Transform|MakeTransform (Transformation|GetActorLocation) "0, 0, 0" "1.000000,1.000000,1.000000") "Undefined" "MultiplyWithRoot" 0 0))

(event Custom|Apply%20Camera%20Shake
  (Camera|PlayWorldCameraShake "/Game/Blueprints/BP_CameraShake.BP_CameraShake_C" "0, 0, 0" 0.0 1e+04))

(event Custom|Check%20Health
  (CallFunction|UpdateHUD)
  (if (== (Variables|Default|GetPlayer%20Health) 0.0)
    (CallFunction|OnDeath))
  (bind _ashud_my_flying_shump (Utilities|Casting|CastToHud_MyFlyingShump (HUD|GetHUD (Variables|Default|GetAs%20Player%20Controller))))
  (Utilities|IsValid (Variables|/Game/Core/Hud_MyFlyingShump.Hud_MyFlyingShump_C|GetPlayer%20Widget _ashud_my_flying_shump)))

(event Custom|OnDeath
  (bind _returnvalue (Actor|GetActorOfClass "/Script/Engine.PlayerStart"))
  (Utilities|IsValid _returnvalue
    (:Is%20Valid
      (bind _returnvalue_2 (Game|SpawnActorfromClass "BP_PlayerPawn_MouseAim_C" (Transformation|GetActorTransform _returnvalue) "Undefined" "MultiplyWithRoot" 0 0))
      (bind _asplayer_controller (Utilities|Casting|CastToPlayerController (Pawn|GetController)))
      (Pawn|Possess _asplayer_controller _returnvalue_2)
      (Actor|DestroyActor)
      (Niagara|SpawnSystematLocation 0 (Transformation|GetActorLocation)))))

(event Custom|FlashRedOverlayMaterial
  (Rendering|Material|SetOverlayMaterial (Variables|Default|GetMesh) "/Game/Materials/M_OverlayWhenHit.M_OverlayWhenHit" :!class /Script/Engine.MeshComponent)
  (Utilities|FlowControl|Delay 0.2)
  (Rendering|Material|SetOverlayMaterial (Variables|Default|GetMesh) 0 :!class /Script/Engine.MeshComponent))

(event Custom|UpdateHUD)

(event Custom|Check%20Lives
  (CallFunction|UpdateHUD)
  (if true
    (CallFunction|OnDeath))
  (bind _ashud_my_flying_shump (Utilities|Casting|CastToHud_MyFlyingShump (HUD|GetHUD (Variables|Default|GetAs%20Player%20Controller))))
  (Utilities|IsValid (Variables|/Game/Core/Hud_MyFlyingShump.Hud_MyFlyingShump_C|GetPlayer%20Widget _ashud_my_flying_shump)))

(event Custom|CheckMissleSupply
  (CallFunction|UpdateHUD)
  (if true
    (CallFunction|BeginFire)
    (bind _ashud_my_flying_shump (Utilities|Casting|CastToHud_MyFlyingShump (HUD|GetHUD (Variables|Default|GetAs%20Player%20Controller))))
    (Utilities|IsValid (Variables|/Game/Core/Hud_MyFlyingShump.Hud_MyFlyingShump_C|GetPlayer%20Widget _ashud_my_flying_shump))))

(event Input|EnhancedActionEvents|EnhancedInputActionIA_MoveForwardBackward
  (params (ActionValue :type Float%20%28double-precision%29) (ElapsedSeconds :type Float%20%28double-precision%29) (TriggeredSeconds :type Float%20%28double-precision%29) (InputAction :type Input%20Action%20Object%20Reference :default "/Game/Inputs/IA_MoveForwardBackward.IA_MoveForwardBackward"))
  (Class|PawnMovementComponent|AddInputVector (Variables|Default|GetFloatingPawnMovement) (Math|Vector|MakeVector ActionValue 0.0 0.0) false))

(event Input|EnhancedActionEvents|EnhancedInputActionIA_MoveRightLeft
  (params (ActionValue :type Float%20%28double-precision%29) (ElapsedSeconds :type Float%20%28double-precision%29) (TriggeredSeconds :type Float%20%28double-precision%29) (InputAction :type Input%20Action%20Object%20Reference :default "/Game/Inputs/IA_MoveRightLeft.IA_MoveRightLeft"))
  (Class|PawnMovementComponent|AddInputVector (Variables|Default|GetFloatingPawnMovement) (Math|Vector|MakeVector 0.0 ActionValue 0.0) false))

(event Input|EnhancedActionEvents|EnhancedInputActionIA_PrimaryFire
  (params (ActionValue :type Boolean) (ElapsedSeconds :type Float%20%28double-precision%29) (TriggeredSeconds :type Float%20%28double-precision%29) (InputAction :type Input%20Action%20Object%20Reference :default "/Game/Inputs/IA_PrimaryFire.IA_PrimaryFire"))
  (bind _arrow (Variables|Default|GetArrow))
  (bind _numberofbulletstospray (Variables|Default|GetNumberOfBulletsToSpray))
  (bind _angleofsprayed_bullets (Variables|Default|GetAngleOfSprayed%20Bullets))
  (bind _primaryfirespawnpoint (Variables|Default|GetPrimaryFireSpawnPoint))
  (bind _returnvalue (Transformation|GetWorldTransform _primaryfirespawnpoint))
  (bind _returnvalue_2 (Math|Vector|GetForwardVector _arrow))
  (bind _returnvalue_3 (Math|Rotator|MakeRotfromX _returnvalue_2))
  (Utilities|FlowControl|Delay 0.2)
  ;[0.15 0.15 0.15 0.5] Shooting Mode 1 (Minigun)
  (switch int (Variables|Default|GetShootingModeIndex)
    (:0
      (Game|SpawnActorfromClass "/Game/Blueprints/BP_Bullet_2D_Player.BP_Bullet_2D_Player_C" (Math|Transform|MakeTransform (.location _returnvalue) (.rotation _returnvalue) "1.000000,1.000000,1.000000") "Undefined" "MultiplyWithRoot" 0 0))
    (:1
      ;[0.15 0.15 0.15 0.5] Shooting Mode 2 (Missiles)
      (bind _isa (Utilities|FlowControl|FlipFlop)
        (:A
          _)
        (:B
          _))
      (Game|SpawnActorfromClass "/Game/Blueprints/BP_PlayerMissle.BP_PlayerMissle_C" (Math|Transform|MakeTransform (.location (Transformation|GetWorldTransform (select _isa (Variables|Default|GetPrimaryFireSpawnPoint3) (Variables|Default|GetPrimaryFireSpawnPoint2)))) (.rotation (Transformation|GetWorldTransform (select _isa (Variables|Default|GetPrimaryFireSpawnPoint3) (Variables|Default|GetPrimaryFireSpawnPoint2)))) "1.000000,1.000000,1.000000") "Undefined" "MultiplyWithRoot" 0 0))
    (:2
      ;[0.15 0.15 0.15 0.5] Optional Shooting Mode (Spray Pattern)
      (Utilities|FlowControl|Delay 0.2)
      (for _index (range 1 (Variables|Default|GetNumberOfBulletsToSpray))
        (Game|SpawnActorfromClass "/Game/Blueprints/BP_Bullet_2D_Player.BP_Bullet_2D_Player_C" (Math|Transform|MakeTransform (Transformation|GetWorldLocation _arrow) (Math|Rotator|MakeRotator (.roll _returnvalue_3) (.pitch _returnvalue_3) (+ (.yaw _returnvalue_3) (Utilities|Operators|Subtract (* _index _angleofsprayed_bullets) (* (Math|Float|Round (* _numberofbulletstospray 0.5)) (Variables|Default|GetAngleOfSprayed%20Bullets)) (Utilities|Select :Index (Math|Integer|%(Integer) _numberofbulletstospray 2) :Option%200 (* _angleofsprayed_bullets 0.5) :Option%201 0.0)))) "1.000000,1.000000,1.000000") "Undefined" "MultiplyWithRoot" 0 0)))))

(event Input|EnhancedActionEvents|EnhancedInputActionIA_LookWithMouse
  (params (ActionValue :type Vector%202D%20Structure) (ElapsedSeconds :type Float%20%28double-precision%29) (TriggeredSeconds :type Float%20%28double-precision%29) (InputAction :type Input%20Action%20Object%20Reference :default "/Game/Inputs/IA_LookWithMouse.IA_LookWithMouse"))
  (Development|PrintString (Utilities|String|ToString(Vector2d) ActionValue)))

(event Collision|EventActorBeginOverlap
  (params (OtherActor :type Actor%20Object%20Reference))
  (Game|Damage|ApplyDamage OtherActor (Variables|Default|GetPlayer%20Health) 0 0))

(event Game|Damage|EventAnyDamage
  (params (Damage :type Float%20%28single-precision%29) (DamageType :type Damage%20Type%20Object%20Reference) (InstigatedBy :type Controller%20Object%20Reference) (DamageCauser :type Actor%20Object%20Reference))
  (bind _output_get (Variables|Default|SetPlayer%20Health (Math|Float|Clamp(Float) (- (Variables|Default|GetPlayer%20Health) Damage) 0.0 (Variables|Default|GetMax%20Health))))
  (CallFunction|ApplyCameraShake)
  (CallFunction|FlashRedOverlayMaterial)
  (CallFunction|CheckHealth)
  (Development|PrintString (Utilities|String|ToString(Float) _output_get)))

(event EventBeginPlay
  (Collision|SetCollisionEnabled (Variables|Default|GetSphere) "NoCollision")
  (Utilities|FlowControl|Delay 0.2)
  (Collision|SetCollisionEnabled (Variables|Default|GetSphere) "QueryAndPhysics")
  (Variables|/Script/Engine.PlayerController|SetbShowMouseCursor (Variables|Default|GetAs%20Player%20Controller) true)
  (Variables|/Script/Engine.PlayerController|SetCurrentMouseCursor (Variables|Default|GetAs%20Player%20Controller) "Crosshairs"))

(event EventPossessed
  (params (NewController :type Controller%20Object%20Reference))
  (bind _asplayer_controller (Utilities|Casting|CastToPlayerController NewController))
  (bind _output_get (Variables|Default|SetAs%20Player%20Controller _asplayer_controller))
  (Input|AddMappingContext (PlayerController|LocalPlayerSubsystems|GetEnhancedInputLocalPlayerSubsystem _output_get) "/Game/Inputs/IMC_PlayeInputs.IMC_PlayeInputs" 0 "(bIgnoreAllPressedKeysUntilRelease=True,bForceImmediately=False,bNotifyUserSettings=False)")
  (CallFunction|CheckHealth))

(event EventTick
  (params (DeltaSeconds :type Float%20%28single-precision%29))
  (Transformation|SetWorldLocation (Variables|Default|GetMouseTarget) (.Location (Collision|BreakHitResult (.HitResult (Class|PlayerController|GetHitResultUnderFingerbyChannel (Variables|Default|GetAs%20Player%20Controller) "Touch1" "TraceTypeQuery1" false)))) false false)
  (Transformation|SetActorRotation (Math|Rotator|MakeRotator 0.0 0.0 (.yaw (Math|Rotator|FindLookatRotation (Transformation|GetActorLocation) (Transformation|GetWorldLocation (Variables|Default|GetMouseTarget)))))))

(event Input|KeyboardEvents|DebugKeyM
  (params (Key :type Key%20Structure :default "None") (ActionValue :type Input%20Action%20Value%20Structure))
  (:Pressed
    (Variables|Default|SetShootingModeIndex (Math|Integer|Clamp(Integer) (+ (Variables|Default|GetShootingModeIndex) 1) 0 2))))

(event Input|KeyboardEvents|DebugKeyN
  (params (Key :type Key%20Structure :default "None") (ActionValue :type Input%20Action%20Value%20Structure))
  (:Pressed
    (Variables|Default|SetShootingModeIndex (Math|Integer|Clamp(Integer) (- (Variables|Default|GetShootingModeIndex) 1) 0 2))))

(fn ConstructionScript)