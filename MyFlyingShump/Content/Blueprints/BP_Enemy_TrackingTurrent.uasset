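; BP_Enemy_TrackingTurrent is an enemy turret that turns on its yaw axis to face player 0.
; From BeginPlay, FireBullet plays the EaseFacePlayer timeline, which restarts itself on finish.
; Each update applies the look-at yaw; RInterpTo gets identical current and target values, so adds no easing.
; Despite its name, FireBullet fires nothing: the BP_2D_E spawn at ShootingDirection is unreachable, and the FacePlayer timer event is empty.
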(event EventBeginPlay
  (|CallParentFunction)
  (CallFunction|FireBullet))

(event EventFacePlayer)

(event EventFireBullet
  (Utilities|Time|SetTimerbyEvent (delegate EventFacePlayer) 0.0)
  (Timeline|EaseFacePlayer PlayFromStart
    (:Update
      (bind _output_get (Variables|Default|SetCurrentYaw (.yaw (Math|Rotator|FindLookatRotation (Transformation|GetActorLocation) (Transformation|GetActorLocation (Game|Player|GetPlayerPawn 0))))))
      (bind _output_get_2 (Variables|Default|SetCurrentYaw (.yaw (Math|Interpolation|RInterpTo (Math|Rotator|MakeRotator 0.0 0.0 (Variables|Default|GetCurrentYaw)) (Math|Rotator|MakeRotator 0.0 0.0 _output_get) (Utilities|Time|GetWorldDeltaSeconds) 2.0))))
      (Transformation|SetActorRotation (Math|Rotator|MakeRotator 0.0 0.0 _output_get_2)))
    (:Finished
      (CallFunction|FireBullet)
      (Timeline|EaseFacePlayer PlayFromStart))))

(fn ConstructionScript
  (|CallParentFunction))