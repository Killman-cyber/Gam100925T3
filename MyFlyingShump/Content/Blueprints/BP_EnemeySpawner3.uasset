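; Enemy spawner Blueprint that repeatedly spawns BP_EnemyC actors along a line between two arrow components.
; On BeginPlay it queues a randomly delayed timer, and each spawn event re-queues it, forming an endless loop with varying intervals.
; Each spawn picks a random Y between the left and right arrows, taking X, Z and rotation from the left arrow.
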(event EventBeginPlay
  (CallFunction|QueueTimer))

(event EventSpawnEnemy
  (bind _arrow_left_side (Variables|Default|GetArrow%20LEFT%20Side))
  (bind _returnvalue (Transformation|GetWorldLocation _arrow_left_side))
  (Game|SpawnActorfromClass "/Game/Blueprints/BP_EnemyC.BP_EnemyC_C" (Math|Transform|MakeTransform (Math|Vector|MakeVector (.x _returnvalue) (Math|Random|RandomFloatinRange (.y _returnvalue) (.y (Transformation|GetWorldLocation (Variables|Default|GetArrow%20RIGHT%20Side)))) (.z _returnvalue)) (Transformation|GetWorldRotation _arrow_left_side) "1.000000,1.000000,1.000000") "Undefined" "MultiplyWithRoot" 0 0)
  (CallFunction|QueueTimer))

(event EventQueueTimer
  (Utilities|Time|SetTimerbyEvent (delegate EventSpawnEnemy) (Math|Random|RandomFloatinRange 5.0 1e+01)))

(fn ConstructionScript
  (|CallParentFunction))