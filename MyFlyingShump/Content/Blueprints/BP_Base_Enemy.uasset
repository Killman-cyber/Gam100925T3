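; Base enemy Blueprint with health, a widget health bar, score feedback and death handling.
; On overlap it deals its current health as damage to the other actor and destroys itself if that actor is tagged "Kill".
; Taking damage adds score, updates the bar, plays a sound and briefly flashes an overlay material.
; At zero health it awards bonus score, explodes, spawns a pickup and, if flagged as last enemy, shows the end screen.
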(event Custom|Check%20Health
  (if (== (Variables|Default|GetHealth) 0.0)
    (Class|BPIMyFlyingShump|AddScore(Message) (Game|GetPlayerController 0) (Variables|Default|GetMax%20Health))
    (CallFunction|OnDeath)))

(event Custom|Flash%20Overlay%20Material
  (bind _mesh (Variables|Default|GetMesh)
    (:then
      (Rendering|Material|SetOverlayMaterial _mesh "/Game/Materials/M_OverlayWhenHit.M_OverlayWhenHit" :!class /Script/Engine.MeshComponent)
      (Utilities|FlowControl|Delay 0.2)
      (bind _mesh_2 (Variables|Default|GetMesh)
        (:then
          (Rendering|Material|SetOverlayMaterial _mesh_2 0 :!class /Script/Engine.MeshComponent))
        (:else)))
    (:else)))

(event EventBeginPlay
  (Variables|Default|SetHealth (Variables|Default|GetMax%20Health)))

(event Collision|EventActorBeginOverlap
  (params (OtherActor :type Actor%20Object%20Reference))
  (Utilities|IsValid OtherActor
    (:Is%20Valid
      (Game|Damage|ApplyDamage OtherActor (Variables|Default|GetHealth) 0 0)
      (Utilities|IsValid OtherActor
        (:Is%20Valid
          (if (Actor|ActorHasTag OtherActor "Kill")
            (Actor|DestroyActor)))))))

(event Game|Damage|EventAnyDamage
  (params (Damage :type Float%20%28single-precision%29) (DamageType :type Damage%20Type%20Object%20Reference) (InstigatedBy :type Controller%20Object%20Reference) (DamageCauser :type Actor%20Object%20Reference))
  (Class|BPIMyFlyingShump|AddScore(Message) (Game|GetPlayerController 0) Damage)
  (Variables|Default|SetHealth (Math|Float|Clamp(Float) (- (Variables|Default|GetHealth) Damage) 0.0 (Variables|Default|GetMax%20Health)))
  (bind _aswbp_enemy_health_bar (Utilities|Casting|CastToWBP_EnemyHealthBar (UserInterface|GetUserWidgetObject (Variables|Default|GetWidget))))
  (Default|SetHealthasPercent _aswbp_enemy_health_bar (Math|Float|SafeDivide (Variables|Default|GetHealth) (Variables|Default|GetMax%20Health)))
  (CallFunction|CheckHealth)
  (Audio|PlaySound2D "/Game/Sci-Fi_Shots_Pack2_Game_Of_Weapons/Cue/SciFi_Shot_P2__122__Cue.SciFi_Shot_P2__122__Cue" 1.0 1.0 0.0 0 0)
  (CallFunction|FlashOverlayMaterial))

(event EventOnDeath
  (bind _returnvalue (Transformation|GetActorTransform))
  (bind _islastenemyoflevel (Variables|Default|GetIsLastEnemyOflevel))
  ;[0.15 0 0 0.5] Viusal And Audio Effects Upon Death
  (Audio|PlaySound2D "/Game/Sci-Fi_Shots_Pack2_Game_Of_Weapons/Cue/SciFi_Shot_P2__109__Cue.SciFi_Shot_P2__109__Cue" 1.0 1.0 0.0 0 0)
  (CallFunction|SpawnExplosion)
  (Game|SpawnActorfromClass (Variables|Default|GetPickupToDropOnDeath) (Math|Transform|MakeTransform (.location _returnvalue) (.rotation _returnvalue) "1.000000,1.000000,1.000000") "Undefined" "MultiplyWithRoot" 0 0)
  (if _islastenemyoflevel
    (Class|BPIMyFlyingShump|ShowEndScreen(Message) (HUD|GetHUD (Game|GetPlayerController 0)) _islastenemyoflevel))
  (Actor|DestroyActor))

(event EventSpawnExplosion
  (Niagara|SpawnSystematLocation "/Game/Particles/FX_EnemyExplosion_System.FX_EnemyExplosion_System" (Transformation|GetActorLocation)))

(fn ConstructionScript)