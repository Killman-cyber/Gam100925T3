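; Base projectile Blueprint that plays a firing sound on BeginPlay and deals missile damage on contact.
; On overlap, it applies DamageMissile to the other actor with no filtering, then destroys itself.
; A FireEnemyMissle event also applies damage and destroys the projectile, but its damage target is unconnected.
; The second sound, apparently meant for impact, is unreachable in both paths, and the graph contains no movement logic.
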(event EventBeginPlay
  (Audio|PlaySound2D "/Game/Sci-Fi_Shots_Pack2_Game_Of_Weapons/Cue/SciFi_Shot_P2__101__Cue.SciFi_Shot_P2__101__Cue" 1.0 1.0 0.0 0 0))

(event EventTick
  (params (DeltaSeconds :type Float%20%28single-precision%29)))

(event Collision|EventActorBeginOverlap
  (params (OtherActor :type Actor%20Object%20Reference))
  (Game|Damage|ApplyDamage OtherActor (Variables|Default|GetDamage%20Missile) 0 0)
  (Actor|DestroyActor))

(event EventFireEnemyMissle
  (Game|Damage|ApplyDamage 0 (Variables|Default|GetDamage%20Missile) 0 0)
  (Actor|DestroyActor))

(fn ConstructionScript)