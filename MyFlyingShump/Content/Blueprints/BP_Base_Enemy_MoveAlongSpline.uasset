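; Base enemy Blueprint that moves the actor along a spline path.
; On BeginPlay it plays a slowed Timeline whose progress samples the spline's world location at constant velocity.
; Each update moves the actor there with sweep enabled, provided the spline reference is valid.
; Rotation logic that orients the mesh from spline vectors is present but never runs, so only position follows the path.
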(event EventBeginPlay
  (|CallParentFunction)
  (Components|Timeline|SetPlayRate (Variables|Default|GetTimeline) 0.1)
  (bind _progress (Timeline|Timeline Play)
    (:Update
      (bind _spline (Variables|Default|GetSpline)
        (:then
          (Transformation|SetActorTransform (Math|Transform|MakeTransform (Spline|GetLocationatTime _spline _progress "World" true) "0, 0, 0" "1.000000,1.000000,1.000000") true))
        (:else)))))

(event Collision|EventActorBeginOverlap
  (params (OtherActor :type Actor%20Object%20Reference))
  (|CallParentFunction OtherActor) ; This node is disabled and will not be called.\nDrag off pins to build functionality.
)

(event EventTick
  (params (DeltaSeconds :type Float%20%28single-precision%29)))

(fn ConstructionScript
  (|CallParentFunction))