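; BP_EnemyC is an enemy actor Blueprint that fires its own 2D bullet type.
; BeginRegularShooting, which nothing in this graph calls, sets a two-second timer on SpawnBullet, with no looping specified.
; SpawnBullet spawns BP_Bullet_2D_EnemyC at the Arrow component's world location and rotation.
; BeginPlay, overlap and Tick are disabled stubs, and the construction script only calls its parent.
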(event Custom|BeginRegularShooting
  (Utilities|Time|SetTimerbyEvent (delegate Custom|SpawnBullet) 2.0))

(event Custom|SpawnBullet
  (bind _arrow (Variables|Default|GetArrow))
  (bind _returnvalue (Transformation|GetWorldTransform _arrow))
  (Game|SpawnActorfromClass "/Game/Blueprints/BP_Bullet_2D_EnemyC.BP_Bullet_2D_EnemyC_C" (Math|Transform|MakeTransform (.location _returnvalue) (.rotation _returnvalue) "1.000000,1.000000,1.000000") "Undefined" "MultiplyWithRoot" 0 0))

(event EventBeginPlay
  (|CallParentFunction) ; This node is disabled and will not be called.\nDrag off pins to build functionality.
)

(event Collision|EventActorBeginOverlap
  (params (OtherActor :type Actor%20Object%20Reference))
  (|CallParentFunction OtherActor) ; This node is disabled and will not be called.\nDrag off pins to build functionality.
)

(event EventTick
  (params (DeltaSeconds :type Float%20%28single-precision%29)))

(fn ConstructionScript
  (|CallParentFunction))