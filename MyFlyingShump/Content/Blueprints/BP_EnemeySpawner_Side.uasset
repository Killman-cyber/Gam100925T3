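; Side enemy spawner actor that repeatedly spawns BP_EnemyB at random points between two arrow markers.
; BeginPlay starts a timer with a random delay of a few seconds, and each spawn re-queues it with a fresh random delay.
; Spawns randomize Y between the left and right arrows, taking X, Z and rotation from the left arrow.
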(event Custom|QueueTimer
  (Utilities|Time|SetTimerbyEvent (delegate Custom|Spawn%20Enemy) (Math|Random|RandomFloatinRange 2.0 6.0) true))

(event Custom|Spawn%20Enemy
  (bind _arrow_left_side (Variables|Default|GetArrow%20LEFT%20Side))
  (bind _returnvalue (Transformation|GetWorldLocation _arrow_left_side))
  (Game|SpawnActorfromClass "/Game/Blueprints/BP_EnemyB.BP_EnemyB_C" (Math|Transform|MakeTransform (Math|Vector|MakeVector (.x _returnvalue) (Math|Random|RandomFloatinRange (.y _returnvalue) (.y (Transformation|GetWorldLocation (Variables|Default|GetArrow%20RIGHT%20Side)))) (.z _returnvalue)) (Transformation|GetWorldRotation _arrow_left_side) "1.000000,1.000000,1.000000") "Undefined" "MultiplyWithRoot" 0 0)
  (CallFunction|QueueTimer))

(event EventBeginPlay
  (CallFunction|QueueTimer))

(fn ConstructionScript)